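; AfterImagesBP is a short-lived afterimage actor that leaves a ghost copy of its Yasuo owner.
; On BeginPlay it applies a dynamic ghost material to its poseable mesh, hides the Blade bone, and copies the owner's mesh scale, rotation and current pose.
; A FadeAway timeline scales the material's starting opacity, then destroys the actor when finished.
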(event EventBeginPlay
  (bind _poseablemesh (Variables|Default|GetPoseableMesh))
  (bind _poseablemesh_2 (Variables|Default|GetPoseableMesh))
  (bind _returnvalue (Rendering|Material|CreateDynamicMaterialInstance "/Game/VFX/JashinGhostMat.JashinGhostMat" "None" "None" :!class /Script/Engine.KismetMaterialLibrary))
  (bind _output_get (Variables|Default|SetDynamicMat _returnvalue))
  (Rendering|Material|SetMaterial _poseablemesh_2 0 _output_get)
  (Rendering|Material|SetMaterial _poseablemesh_2 1 _output_get)
  (Rendering|Material|SetMaterial _poseablemesh_2 2 _output_get)
  (Rendering|Material|SetMaterial _poseablemesh_2 3 _output_get)
  (Components|SkinnedMesh|HideBonebyName (Variables|Default|GetPoseableMesh) "Blade" "PBO_None")
  (bind _asyasuo (Utilities|Casting|CastToYasuo (Components|GetOwner)))
  (Transformation|SetWorldScale3D _poseablemesh (Transformation|GetWorldScale (Variables|/Script/Engine.Character|GetMesh _asyasuo)))
  (Transformation|SetWorldRotation _poseablemesh (Transformation|GetWorldRotation (Variables|/Script/Engine.Character|GetMesh _asyasuo)) false false)
  (Class|PoseableMeshComponent|CopyPosefromSkeletalComponent (Variables|Default|GetPoseableMesh) (Variables|/Script/Engine.Character|GetMesh _asyasuo))
  (bind _returnvalue_2 (Rendering|Material|GetScalarParameterValue (Variables|Default|GetDynamicMat) "Opacity" :!class /Script/Engine.MaterialInstanceDynamic))
  (Variables|Default|SetOpacityMax _returnvalue_2)
  (bind _opacity (Timeline|Fade%20Away Play)
    (:Update
      (Rendering|Material|SetScalarParameterValue (Variables|Default|GetDynamicMat) "Opacity" (* _opacity (Variables|Default|GetOpacityMax)) :!class /Script/Engine.MaterialInstanceDynamic))
    (:Finished
      (Actor|DestroyActor))))

(fn ConstructionScript)